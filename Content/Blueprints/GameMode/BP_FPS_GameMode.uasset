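; FPS game mode that runs a timed drone-clearing round and shows its status on a GameMode HUD widget.
; A Tick-driven session state machine locks input during warm-up, then counts down the game timer, turning it red near the end.
; Drones are counted at BeginPlay; DroneDeath decrements the count and triggers a win if the player is alive.
; Running out of time or PlayerDies ends the round with an announcement and disabled input.
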(event `self.ReceiveBeginPlay`
  ;[1 1 1] Add GameMode HUD
  (bind _returnvalue (`|CreateWidget` "/Game/Blueprints/HUD/WBP_GameModeHUD.WBP_GameModeHUD_C"))
  (bind _output_get (set `self.GameMode_HUD` _returnvalue))
  (`UserWidget.AddToViewport` _output_get 0)
  (`TextBlock.SetText` (`/Game/Blueprints/HUD/WBP_GameModeHUD.Announcement` _output_get) "Clear the drones from the area!")
  (`TextBlock.SetText` (`/Game/Blueprints/HUD/WBP_GameModeHUD.TimeText` _output_get) (`self.TimeRemainingFormat`))
  (`self.CheckTotalDrones`))

(event `self.ReceiveTick`
  (params (DeltaSeconds :type "Float (single-precision)"))
  (switch `/Game/Blueprints/GameMode/E_SessionState` (`self.SessionState`)
    (:`NewEnumerator0`
      (`self.DisablePlayerInput`)
      (`self.UpdateWarmUpTimer`))
    (:`NewEnumerator1`
      (`self.UpdateGameTimer` DeltaSeconds)
      (`self.CheckOutOfTime`))
    (:`NewEnumerator2`
      (`self.PlayerIsOutOfTime`))))

(fn `CheckOutOfTime`
  (if (<= (`self.GameTimer`) 0.0)
    (set `self.SessionState` "NewEnumerator2")))

(fn `CheckTotalDrones`
  (bind _outactors (`GameplayStatics.GetAllActorsOfClass` "/Game/Blueprints/Drone/BP_Drone.BP_Drone_C"))
  (set `self.Drones` (`KismetArrayLibrary.Array_Length` _outactors)))

(fn `CountWarmUpTimerInt64`
  (returns (ReturnValue :type Integer64))
  (return (`KismetMathLibrary.FCeil64` (- (`self.WarmUpTime`) (`KismetSystemLibrary.GetGameTimeInSeconds`)))))

(fn `DisablePlayerInput`
  (bind _returnvalue (`GameplayStatics.GetPlayerCharacter` 0))
  (bind _asplayer_controller (cast `PlayerController` (`Pawn.GetController` _returnvalue)))
  (`self.DisableInput` _returnvalue _asplayer_controller))

(fn `DroneDeath`
  (bind _result (`/Engine/EditorBlueprintResources/StandardMacros.DecrementInt` (`self.Drones`))
    (:`  `
      (if (<= _result 0)
        (`self.PlayerWins`)))))

(fn `PlayerDies`
  (bind _gamemode_hud (`self.GameMode_HUD`))
  (set `self.SessionState` "NewEnumerator3")
  (`TextBlock.SetText` (`/Game/Blueprints/HUD/WBP_GameModeHUD.Announcement` _gamemode_hud) "You died!")
  (`TextBlock.SetText` (`/Game/Blueprints/HUD/WBP_GameModeHUD.TimeText` _gamemode_hud) "00:00")
  (`self.DisablePlayerInput`))

(fn `PlayerIsOutOfTime`
  (bind _returnvalue (`GameplayStatics.GetPlayerCharacter` 0))
  (bind _gamemode_hud (`self.GameMode_HUD`))
  (bind _asplayer_controller (cast `PlayerController` (`Pawn.GetController` _returnvalue)))
  (`self.DisableInput` _returnvalue _asplayer_controller)
  (`TextBlock.SetText` (`/Game/Blueprints/HUD/WBP_GameModeHUD.TimeText` _gamemode_hud) "00:00")
  (`TextBlock.SetText` (`/Game/Blueprints/HUD/WBP_GameModeHUD.Announcement` _gamemode_hud) "Out of time! Drones are now killing civilians"))

(fn `PlayerWins`
  (bind _asbp_fps_character (cast `/Game/Blueprints/Character/BP_FPS_Character` (`GameplayStatics.GetPlayerCharacter` 0)))
  (if (> (`/Game/Blueprints/Shared/BP_HealthComponent.Health` (`/Game/Blueprints/Character/BP_FPS_Character.HealthComponent` _asbp_fps_character)) 0.0)
    (set `self.SessionState` "NewEnumerator4")
    (`TextBlock.SetText` (`/Game/Blueprints/HUD/WBP_GameModeHUD.Announcement` (`self.GameMode_HUD`)) "Congratulations! You cleared the drone threat!")
    (`self.DisablePlayerInput`)))

(fn `StartGame`
  (bind _returnvalue (`GameplayStatics.GetPlayerCharacter` 0))
  (set `self.SessionState` "NewEnumerator1")
  (bind _asplayer_controller (cast `PlayerController` (`Pawn.GetController` _returnvalue)))
  (`self.EnableInput` _returnvalue _asplayer_controller)
  (`TextBlock.SetText` (`/Game/Blueprints/HUD/WBP_GameModeHUD.WarmUpText` (`self.GameMode_HUD`)) "")
  (`TextBlock.SetText` (`/Game/Blueprints/HUD/WBP_GameModeHUD.Announcement` (`self.GameMode_HUD`)) ""))

(fn `TimeRemainingFormat`
  (returns (`Formatted Time` :type Text))
  (bind _returnvalue (`KismetMathLibrary.FFloor64` (/ (`self.GameTimer`) 60.0)))
  (return (`|FormatText` "{Minutes}:{Seconds}" (`KismetTextLibrary.Conv_Int64ToText` _returnvalue false true 2 2) (`KismetTextLibrary.Conv_DoubleToText` (- (`self.GameTimer`) (* (`KismetMathLibrary.Conv_Int64ToDouble` _returnvalue) 60.0)) "HalfToEven" false true 2 2 0 0))))

(fn `UpdateGameTimer`
  (params (DeltaTime :type "Float (double-precision)"))
  (bind _timetext (`/Game/Blueprints/HUD/WBP_GameModeHUD.TimeText` (`self.GameMode_HUD`)))
  (bind _output_get (set `self.GameTimer` (- (`self.GameTimer`) DeltaTime)))
  (`TextBlock.SetText` _timetext (`self.TimeRemainingFormat`))
  (if (<= _output_get 10.0)
    (`TextBlock.SetColorAndOpacity` _timetext (make `SlateColor` (struct :`R` 0.796875 :`A` 1.0)))))

(fn `UpdateWarmUpTimer`
  (bind _returnvalue (`self.CountWarmUpTimerInt64`))
  (`TextBlock.SetText` (`/Game/Blueprints/HUD/WBP_GameModeHUD.WarmUpText` (`self.GameMode_HUD`)) (`KismetTextLibrary.Conv_Int64ToText` _returnvalue))
  (if (<= _returnvalue 0)
    (`self.StartGame`)))

(fn `UserConstructionScript`)
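; BP_FPS_Character is a first-person player character Blueprint that handles basic movement, look and jump input.
; Axis events move it along the actor's forward and right vectors and feed controller yaw and pitch for looking.
; Sprint doubles the CharacterMovement max walk speed on press and halves it on release, scaling the current value rather than storing a base speed.
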(event `InputAxis|MoveForward`
  (params (AxisValue :type "Float (single-precision)"))
  ;[1 1 1] Character Controls
  ;;[1 1 1] Character Movement
  (`self.AddMovementInput` (`self.GetActorForwardVector`) AxisValue))

(event `InputAxis|Turn`
  (params (AxisValue :type "Float (single-precision)"))
  ;[1 1 1] Character Controls
  ;;[1 1 1] Character Look
  (`self.AddControllerYawInput` AxisValue))

(event `InputAction|Sprint`
  (params (Key :type "Key Structure"))
  (bind _charactermovement (`self.CharacterMovement`))
  (:`Pressed`
    (set `CharacterMovementComponent.MaxWalkSpeed` (* 2.0 (`CharacterMovementComponent.MaxWalkSpeed` _charactermovement)) _charactermovement))
  (:`Released`
    (set `CharacterMovementComponent.MaxWalkSpeed` (/ (`CharacterMovementComponent.MaxWalkSpeed` _charactermovement) 2.0) _charactermovement)))

(event `InputAxis|LookUp`
  (params (AxisValue :type "Float (single-precision)"))
  ;[1 1 1] Character Controls
  ;;[1 1 1] Character Look
  (`self.AddControllerPitchInput` AxisValue))

(event `InputAxis|MoveRight`
  (params (AxisValue :type "Float (single-precision)"))
  ;[1 1 1] Character Controls
  ;;[1 1 1] Character Movement
  (`self.AddMovementInput` (`self.GetActorRightVector`) AxisValue))

(event `InputAction|Jump`
  (params (Key :type "Key Structure"))
  ;[1 1 1] Character Controls
  ;;[1 1 1] Character Jump
  (:`Pressed`
    (`self.Jump`)))

(event `self.ReceiveTick`
  (params (DeltaSeconds :type "Float (single-precision)")))

(fn `UserConstructionScript`)
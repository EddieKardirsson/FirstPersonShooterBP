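; Ammo pickup actor that spins and adds its Ammo value to an overlapping BP_FPS_Character.
; Tick turns the Sphere by a hardcoded yaw step per frame, independent of delta time and the RotationSpeed input.
; Sphere overlap calls AddAmmoToPlayer, which casts the other actor, increases its ammo and plays a 2D equip sound.
; The pickup then destroys itself, even when the overlapping actor is not that character.
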(event `self.ReceiveTick`
  (params (DeltaSeconds :type "Float (single-precision)"))
  (bind _sphere (`self.Sphere`))
  (`SceneComponent.K2_SetRelativeRotation` _sphere (`/Game/Blueprints/Shared/BPL_SharedFunctionLibrary.UpdateRotation` _sphere (`self.RotationSpeed`)) false false))

(event `self.Sphere.OnComponentBeginOverlap`
  (params (OverlappedComponent :type "PrimitiveComponent Object Reference") (OtherActor :type "Actor Object Reference") (OtherComp :type "PrimitiveComponent Object Reference") (OtherBodyIndex :type Integer) (bFromSweep :type Boolean) (SweepResult :type "HitResult Structure (by ref)"))
  (`self.AddAmmoToPlayer` OtherActor)
  (`self.K2_DestroyActor`))

(fn `AddAmmoToPlayer`
  (params (Object :type "Object Object Reference"))
  (bind _asbp_fps_character (cast `/Game/Blueprints/Character/BP_FPS_Character` Object))
  (set `/Game/Blueprints/Character/BP_FPS_Character.Ammo` (+ (`/Game/Blueprints/Character/BP_FPS_Character.Ammo` _asbp_fps_character) (`self.Ammo`)) _asbp_fps_character)
  (`GameplayStatics.PlaySound2D` "/Game/Assets/Sounds/Ammo/sw_AmmoEquip.sw_AmmoEquip" 1.0 1.0 0.0 null null))

(fn `UpdateRotation`
  (returns (Sphere :type "SphereComponent Object Reference") (ReturnValue :type "Rotator Structure"))
  (bind _sphere (`self.Sphere`))
  (bind (_relativerotation_roll _relativerotation_pitch _relativerotation_yaw) (`KismetMathLibrary.BreakRotator` (`SceneComponent.RelativeRotation` _sphere)))
  (return _sphere (`KismetMathLibrary.MakeRotator` 0.0 0.0 (+ -1.25 _relativerotation_yaw))))

(fn `UserConstructionScript`)
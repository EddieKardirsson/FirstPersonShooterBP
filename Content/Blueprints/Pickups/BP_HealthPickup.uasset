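; Health pickup actor that restores health to the player's BP_FPS_Character when it touches the pickup.
; Sphere overlap calls AddHealthToPlayer, which casts the other actor and applies an amount from the Health variable through ChangeHealth, then plays a 2D sound and destroys the pickup.
; Despite its name, IsHealthAtMaximum returns true when health is below maximum, so full-health players leave the pickup in place.
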(event `self.Sphere.OnComponentBeginOverlap`
  (params (OverlappedComponent :type "PrimitiveComponent Object Reference") (OtherActor :type "Actor Object Reference") (OtherComp :type "PrimitiveComponent Object Reference") (OtherBodyIndex :type Integer) (bFromSweep :type Boolean) (SweepResult :type "HitResult Structure (by ref)"))
  (`self.AddHealthToPlayer` OtherActor))

(fn `AddHealthToPlayer`
  (params (Object :type "Object Object Reference"))
  (bind _asbp_fps_character (cast `/Game/Blueprints/Character/BP_FPS_Character` Object))
  (if (`self.IsHealthAtMaximum` _asbp_fps_character)
    (bind _result (`/Engine/EditorBlueprintResources/StandardMacros.NegateFloat` (`self.Health`))
      (:`  `
        (`/Game/Blueprints/Character/BP_FPS_Character.ChangeHealth` _asbp_fps_character _result)
        (`GameplayStatics.PlaySound2D` "/Game/Assets/Sounds/Health/sw_Pickup_Health.sw_Pickup_Health" 1.0 1.0 0.0 null null)
        (`self.K2_DestroyActor`)))))

(fn `IsHealthAtMaximum`
  (params (Player :type "/Game/Blueprints/Character/BP_FPS_Character Object Reference"))
  (returns (ReturnValue :type Boolean))
  (return (< (`/Game/Blueprints/Shared/BP_HealthComponent.Health` (`/Game/Blueprints/Character/BP_FPS_Character.HealthComponent` Player)) (`/Game/Blueprints/Character/BP_FPS_Character.MaxHealth` Player))))

(fn `UserConstructionScript`)